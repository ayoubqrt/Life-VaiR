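; BP_Cloud is a floating assistant that follows the player via PawnSensing and offers hints from a dialog DataTable.
; It binds every BaseMachine's overlap events, jumping above an entered machine and counting seconds per machine type with a looping timer.
; Timed checks trigger help lines based on machine visits, time and success.
; Machine success loads the save and, for one type, prints agriculture NOx emissions.
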(event OnSeePawn(PawnSensing)
  (params (Pawn :type Pawn%20Object%20Reference))
  (if (Variables|PlayerData|GetIsPlayerOnMachine)
    ;[1 1 1] Rotate to look at the player when he is on machine
    (Transformation|SetActorRotation (Math|Rotator|MakeRotator 0.0 0.0 (.Z (Class|KismetMathLibrary|BreakVector3f (Pawn|GetNavAgentLocation Pawn)))))
    (else
      ;[1 1 1] Move to player
      (AI|AIMoveTo self "0, 0, 0" Pawn 3e+02 false))))

(event Custom|OnMachineOverlap
  (params (OverlappedActor :type Actor%20Object%20Reference) (OtherActor :type Actor%20Object%20Reference))
  ;[1 1 1] Listen Machine Overlap event
  (if (== OverlappedActor (Game|GetPlayerCharacter 0))
    _
    (else
      _))
  (bind _asbase_machine (Utilities|Casting|CastToBaseMachine OverlappedActor))
  (bind _returnvalue (Utilities|Time|SetTimerbyFunctionName 0 "Increment" 1.0 true))
  (bind _output_get (Variables|PlayerData|SetLastMachineOverlappedByPlayer _asbase_machine))
  (Variables|PlayerData|SetIsPlayerOnMachine true)
  (CallFunction|Animations)
  (Transformation|SetActorLocation (Math|Vector|MakeVector (.X (Class|KismetMathLibrary|BreakVector3f (Transformation|GetActorLocation _output_get))) (.Y (Class|KismetMathLibrary|BreakVector3f (Transformation|GetActorLocation _output_get))) 1e+03) false false) ; Teleport cube on top of the machine
)

(event Custom|DialogNoMachineStepped
  ;[1 1 1] Help player to go on a machine when no machines stepped after 1 second
  (Utilities|IsValid (Variables|PlayerData|GetLastMachineOverlappedByPlayer)
    (:Is%20Not%20Valid
      (bind _returnvalue (Utilities|GetDataTableRow "/Game/Core/CloudAssistant/DT_Cloud_Dialogs.DT_Cloud_Dialogs" "NoMachinesStepped")
        (:then
          (Development|PrintString (Utilities|String|ToString(Text) (Utilities|Struct|BreakS_Cloud_Dialogs _returnvalue)))
          (Audio|PlaySound2D "/Game/Core/CloudAssistant/NoMachinesStepped.NoMachinesStepped" 1.0 1.0 0.0 0 0))))))

(event Custom|OnMachineEndOverlap
  (params (OverlappedActor :type Actor%20Object%20Reference) (OtherActor :type Actor%20Object%20Reference))
  ;[1 1 1] Listen Machine Overlap event
  (if (== OverlappedActor OtherActor)
    _
    (else
      _))
  (Utilities|Time|ClearandInvalidateTimerbyHandle (stale Custom|OnMachineOverlap _returnvalue))
  (Variables|PlayerData|SetIsPlayerOnMachine false))

(event Custom|Increment
  (bind _timepassedonmachines (Variables|PlayerData|GetTimePassedOnMachines))
  (bind _lastmachineoverlappedbyplayer (Variables|PlayerData|GetLastMachineOverlappedByPlayer))
  (bind _machinetype (Variables|/Game/Core/Riddles/BaseMachine.BaseMachine_C|GetMachineType _lastmachineoverlappedbyplayer))
  ;[1 1 1] Increment time passed on current machine
  (bind _result (Math|Integer|IncrementInt (.Value (Utilities|Map|Find _timepassedonmachines _machinetype)))
    (:%20%20
      (Utilities|Map|Add _timepassedonmachines _machinetype _result)
      (Rendering|Components|TextRender|SetText (Variables|Default|GetDialog) (Utilities|Text|ToText(String) (Utilities|String|Append (Utilities|String|ToString(Text) (Utilities|Text|ToText(Integer) _result)) (Utilities|String|ToString(Text) (Utilities|Text|ToText(String) (Utilities|String|EnumtoString _machinetype)))))))))

(event Custom|CheckIfNeedToDialog
  (bind _lastmachineoverlappedbyplayer (Variables|PlayerData|GetLastMachineOverlappedByPlayer))
  ;[1 1 1] Help the player if he has passed more than 5 seconds on the current machine
  (Utilities|FlowControl|Sequence
    (:then_0
      (Utilities|IsValid _lastmachineoverlappedbyplayer
        (:Is%20Valid
          (if (and (not (Variables|/Game/Core/Riddles/BaseMachine.BaseMachine_C|GetSucceeded _lastmachineoverlappedbyplayer)) (> 10 (.ReturnValue (Utilities|Map|Find (Variables|PlayerData|GetTimePassedOnMachines) (Variables|/Game/Core/Riddles/BaseMachine.BaseMachine_C|GetMachineType _lastmachineoverlappedbyplayer)))))
            (bind _returnvalue (Utilities|GetDataTableRow "/Game/Core/CloudAssistant/DT_Cloud_Dialogs.DT_Cloud_Dialogs" "Long_Time_Didnt_Played")
              (:then
                (Development|PrintString (Utilities|String|ToString(Text) (Utilities|Struct|BreakS_Cloud_Dialogs _returnvalue)))))))))))

(event Custom|Animations
  ;[1 1 1] Animate the cube when the player is on a machine
  (bind _floatonmachine (Timeline|FloatOnMachine Play)
    (:Update
      (Transformation|SetRelativeTransform (Variables|Default|GetCube) (Math|Transform|MakeTransform _floatonmachine "0, 0, 0" "1.000000,1.000000,1.000000") false false))))

(event Custom|CustomEvent
  (params (Machine%20Type :type E_MachineTypes%20Enum :default "NewEnumerator0"))
  ;[1 1 1] Read game data when machine is succedded
  (bind _returnvalue (SaveGame|LoadGamefromSlot "CurrentGame"))
  (bind _asbp_save_territory_data (Utilities|Casting|CastToBP_SaveTerritoryData _returnvalue))
  (if (Utilities|Enum|Equal(Enum) Machine%20Type "NewEnumerator0")
    (Development|PrintString (Utilities|String|ToString(Float) (.Emi_NOx (Utilities|Struct|BreakS_Territory_Emissions_SectorSpecific (Variables|/Game/Core/BP_SaveTerritoryData.BP_SaveTerritoryData_C|GetSelected%20Territory%20Emissions%20Agriculture _asbp_save_territory_data)))))))

(event EventBeginPlay
  (Utilities|FlowControl|Sequence
    (:then_0
      ;[1 1 1] Listen Machine Overlap event
      (bind _outactors (Actor|GetAllActorsOfClass "/Game/Core/Riddles/BaseMachine.BaseMachine_C"))
      (for _array_element _outactors
        (Utilities|FlowControl|Sequence
          (:then_0
            (Collision|BindEventtoOnActorBeginOverlap _array_element (delegate Custom|OnMachineOverlap))
            (EventDispatchers|BindEventtoSuccessStateUpdate _array_element (delegate Custom|CustomEvent)))
          (:then_1
            (Collision|BindEventtoOnActorEndOverlap _array_element (delegate Custom|OnMachineEndOverlap))))))
    (:then_1
      ;[1 1 1] Floating animation
      (bind _newtrack_0 (Timeline|Timeline Play)
        (:Update
          (Transformation|SetRelativeTransform (Variables|Default|GetCube) (Math|Transform|MakeTransform _newtrack_0 "0, 0, 0" "1.000000,1.000000,1.000000") false false))))
    (:then_2
      ;[1 1 1] Print hello world
      (bind _returnvalue (Utilities|GetDataTableRow "/Game/Core/CloudAssistant/DT_Cloud_Dialogs.DT_Cloud_Dialogs" "Game_Start")
        (:then
          (Rendering|Components|TextRender|SetText (Variables|Default|GetDialog) (Utilities|Struct|BreakS_Cloud_Dialogs _returnvalue)))))
    (:then_3
      ;[1 1 1] Timers
      (Utilities|Time|SetTimerbyFunctionName 0 "DialogNoMachineStepped" 1.0)
      (Utilities|Time|SetTimerbyFunctionName 0 "CheckIfNeedToDialog" 5.0 true))))

(event Collision|EventActorBeginOverlap
  (params (OtherActor :type Actor%20Object%20Reference)))

(event EventTick
  (params (DeltaSeconds :type Float%20%28single-precision%29)))

(fn ConstructionScript)