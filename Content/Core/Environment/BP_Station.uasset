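; Station hub actor that shows the saved territory's climate and emissions data and tracks progress across the environmental machines.
; BeginPlay fills bridge screens and per-machine widgets from the save, starts audio and sets bad smog.
; The launch button has the game mode set up riddles and advances the screens.
; Each machine success validates its widget, greens its ground material and blends smog toward clear by the succeeded-to-enabled ratio.
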(event Custom|Setup%20riddles
  (bind _launchgamebutton_ref (Variables|ObjectReference|GetLaunchGameButton%20Ref))
  (Development|PrintString "Setup riddles" true true "(R=1.000000,G=0.455150,B=0.222579,A=1.000000)" 4.0 "Setup ")
  (Default|SetupAllRiddles (Variables|ObjectReference|GetGame%20Mode%20Ref))
  (Audio|PlaySoundatLocation "/Game/FX/SFX/Cues/SC_LaunchGame.SC_LaunchGame" (Transformation|GetWorldLocation (Variables|Default|GetBP_LaunchGame)) "0, 0, 0" 1.0 1.0 0.0 0 0 0 0)
  (Default|DisableButton (Variables|ObjectReference|GetLaunchGameButton%20Ref))
  ;[0.1146 0.08949 0.1001] Update the widgets to go to the next screen on button pushed
  (Default|NextWidgetIndex (Variables|ObjectReference|GetBridge%20Scanner%20Status%20Ref))
  (Default|NextWidgetIndex (Variables|ObjectReference|GetAs%20W%20Bridge%20Climate%20Data))
  (Default|NextWidgetIndex (Variables|ObjectReference|GetAs%20W%20Bridge%20Machine%20Screen))
  (Default|LaunchAnalysisandShowResults (Variables|ObjectReference|GetMainScreen%20ref))
  ;[0 0 0] Disable main button
  (Default|Glow _launchgamebutton_ref false)
  (Default|DisableButton _launchgamebutton_ref)
  (Default|ControlButtonGlow _launchgamebutton_ref false 0.0))

(event Custom|Handle%20Machine%20Success
  (params (Machine%20Type :type E_MachineTypes%20Enum :default "NewEnumerator0"))
  (bind _badsituationfog (Variables|SmogManagement|GetBadSituationFog))
  (bind _goodsituationfog (Variables|SmogManagement|GetGoodSituationFog))
  ;[0 0.3385 0.018] Machine succeeded
  (Utilities|FlowControl|Sequence
    (:then_0
      (Math|Integer|IncrementInt (Variables|Default|GetNumber%20of%20Succeeded%20machines)))
    (:then_1
      ;[0 0 0] Update Smog Machine State Change
      (bind _alpha (SmogManagement|ComputeAlpha))
      (bind _output_get (Variables|SmogManagement|SetCurrent%20Smog%20 (Utilities|Struct|MakeBP_SmogSettings (Math|Float|Lerp (.fogdensity _badsituationfog) (.fogdensity _goodsituationfog) _alpha) (Math|Float|Lerp (.fogfalloff _badsituationfog) (.fogfalloff _goodsituationfog) _alpha) (Class|KismetMathLibrary|LinearColorLerpUsingHSV (.fogscatteringcolor _badsituationfog) (.fogscatteringcolor _goodsituationfog) _alpha) 1.0)))
      (CallFunction|UpdateSmogAppearance _output_get))
    (:then_2
      (switch Utilities|FlowControl|Switch|SwitchonE_MachineTypes Machine%20Type
        (:NewEnumerator0
          (Default|SetMachineStatusLogotoValid (Variables|MachineStateWidgets|GetIndustryMachineWidget%20%20ref))
          (bind _returnvalue (Rendering|Material|CreateDynamicMaterialInstance (Variables|Default|Getground) 3 0 "residential " :!class /Script/Engine.PrimitiveComponent)))
        (:NewEnumerator1
          (Default|SetMachineStatusLogotoValid (Variables|MachineStateWidgets|GetEnergyMachineWidget%20ref))
          (bind _returnvalue_2 (Rendering|Material|CreateDynamicMaterialInstance (Variables|Default|Getground) 4 0 "residential " :!class /Script/Engine.PrimitiveComponent)))
        (:NewEnumerator2
          (Default|SetMachineStatusLogotoValid (Variables|MachineStateWidgets|GetResidentialMachineWidget%20%20ref))
          (bind _returnvalue_3 (Rendering|Material|CreateDynamicMaterialInstance (Variables|Default|Getground) 5 0 "residential " :!class /Script/Engine.PrimitiveComponent)))
        (:NewEnumerator3
          (Default|SetMachineStatusLogotoValid (Variables|MachineStateWidgets|GetMobilityMachineWidget%20ref))
          (bind _returnvalue_4 (Rendering|Material|CreateDynamicMaterialInstance (Variables|Default|Getground) 2 0 "mobility " :!class /Script/Engine.PrimitiveComponent)))
        (:NewEnumerator4
          (Default|SetMachineStatusLogotoValid (Variables|MachineStateWidgets|GetAgriMachineWidget%20ref))
          (bind _returnvalue_5 (Rendering|Material|CreateDynamicMaterialInstance (Variables|Default|Getground) 6 0 "agri " :!class /Script/Engine.PrimitiveComponent))))
      (Rendering|Material|SetVectorParameterValue _returnvalue_3 "Emission Color" "(R=0.012628,G=0.434028,B=0.000000,A=1.000000)" :!class /Script/Engine.MaterialInstanceDynamic))))

(event Custom|Analyze%20Button%20pushed
  (params (Button :type BP%20Push%20Button%20Object%20Reference))
  (CallFunction|SetupRiddles))

(event EventBeginPlay
  (bind _defaultsceneroot (Variables|Default|GetDefaultSceneRoot))
  (bind _persistentgamedataref (Variables|Objectreference|GetPersistentGameDataRef))
  (bind _launchgamebutton_ref (Variables|ObjectReference|GetLaunchGameButton%20Ref))
  (bind _persistentgamedataref_2 (Variables|Objectreference|GetPersistentGameDataRef))
  (bind _returnvalue (Transformation|GetWorldLocation _defaultsceneroot))
  (CallFunction|DefineReferences)
  ;[0 0 0] Init screen with territory data
  (Default|InitializeDashboard (Variables|ObjectReference|GetMainScreen%20ref) _persistentgamedataref_2)
  (Default|InitClimateImpactDashboard (Variables|ObjectReference|GetAs%20W%20Bridge%20Climate%20Data) (Variables|/Game/Core/BP_SaveTerritoryData.BP_SaveTerritoryData_C|GetSelected%20Territory%20Other%20Impact _persistentgamedataref_2))
  (Default|Glow _launchgamebutton_ref true)
  (EventDispatchers|BindEventtoButtonPushed _launchgamebutton_ref (delegate Custom|Analyze%20Button%20pushed))
  ;[0 0 0] Define basic sound mix
  (Class|GameplayStatics|SetBaseSoundMix "/Game/FX/SFX/SCM_StationBase.SCM_StationBase") ; Load base sound mix
  (Audio|PlaySoundatLocation "/Game/FX/SFX/Cues/SC_StationEngine.SC_StationEngine" _returnvalue "0, 0, 0" 1.0 1.0 0.0 0 0 0 0)
  (Audio|PlaySoundatLocation "/Game/FX/SFX/Cues/SC_RearPropeller.SC_RearPropeller" (Transformation|GetWorldLocation (Variables|Default|GetStation_rear_propeller)) "0, 0, 0" 1.0 1.0 0.0 0 0 0 0)
  (Audio|PlaySoundatLocation "/Game/FX/SFX/Cues/SC_ResolvingMusic.SC_ResolvingMusic" _returnvalue "0, 0, 0" 1.0 1.0 0.0 0 0 0 0)
  ;[0 0 0 1 13] Begin call to setup fog (random machine)
  (CallFunction|UpdateSmogAppearance (Variables|SmogManagement|GetBadSituationFog))
  (bind _outactors (Actor|GetAllActorsOfClass "/Game/Core/Riddles/BaseMachine.BaseMachine_C"))
  (bind _output_get (Variables|Default|SetMachines _outactors))
  ;[0 0 0] Widgets Setup
  (for _array_element _output_get
    (bind (_enabled _succeeded _machinetype) (Default|GetMachineState _array_element))
    (if _enabled
      (Math|Integer|IncrementInt (Variables|Default|GetNumber%20of%20enables%20machines)
        (:%20%20
          _)))
    (switch Utilities|FlowControl|Switch|SwitchonE_MachineTypes _machinetype
      (:NewEnumerator0
        (CallFunction|UpdateMachineStatusWidget (Variables|MachineStateWidgets|GetIndustryMachineWidget%20%20ref) _succeeded "Industry Machine" (Variables|/Game/Core/BP_SaveTerritoryData.BP_SaveTerritoryData_C|GetSelected%20Territory%20Emissions%20Industry _persistentgamedataref)))
      (:NewEnumerator1
        (CallFunction|UpdateMachineStatusWidget (Variables|MachineStateWidgets|GetEnergyMachineWidget%20ref) _succeeded "Energy Production Machine" (Variables|/Game/Core/BP_SaveTerritoryData.BP_SaveTerritoryData_C|GetSelected%20Territory%20Emissions%20Energy _persistentgamedataref)))
      (:NewEnumerator2
        (CallFunction|UpdateMachineStatusWidget (Variables|MachineStateWidgets|GetResidentialMachineWidget%20%20ref) _succeeded "Residential Machine" (Variables|/Game/Core/BP_SaveTerritoryData.BP_SaveTerritoryData_C|GetSelected%20Territory%20Emissions%20Residential _persistentgamedataref)))
      (:NewEnumerator3
        (CallFunction|UpdateMachineStatusWidget (Variables|MachineStateWidgets|GetMobilityMachineWidget%20ref) _succeeded "Mobility Machine" (Variables|/Game/Core/BP_SaveTerritoryData.BP_SaveTerritoryData_C|GetSelected%20Territory%20Emissions%20Transport _persistentgamedataref)))
      (:NewEnumerator4
        (CallFunction|UpdateMachineStatusWidget (Variables|MachineStateWidgets|GetAgriMachineWidget%20ref) _succeeded "Agriculture Machine" (Variables|/Game/Core/BP_SaveTerritoryData.BP_SaveTerritoryData_C|GetSelected%20Territory%20Emissions%20Agriculture _persistentgamedataref))))
    (EventDispatchers|BindEventtoSuccessStateUpdate _array_element (delegate Custom|Handle%20Machine%20Success))))

(event Custom|Update%20Smog%20Appearance
  (params (Parameters :type BP%20Smog%20Settings%20Structure))
  (bind _smog (Variables|Default|GetSmog))
  (Class|ExponentialHeightFogComponent|SetFogDensity _smog (.fogdensity Parameters))
  (Class|ExponentialHeightFogComponent|SetFogHeightFalloff _smog (.fogfalloff Parameters))
  (Class|ExponentialHeightFogComponent|SetFogInscatteringColor _smog (.fogscatteringcolor Parameters))
  (Class|ExponentialHeightFogComponent|SetFogMaxOpacity _smog (.fogopacity Parameters)))

(event EventTick
  (params (DeltaSeconds :type Float%20%28single-precision%29))
  ;[0.1927 0 0.03534] Rotation of the rear propeller
  (bind _rotation (Timeline|Timeline Play)
    (:Update
      (Transformation|SetRelativeRotation (Variables|Default|GetStation_rear_propeller) (Math|Rotator|MakeRotator _rotation 0.0 0.0) false false))))

(fn ConstructionScript
  (CallFunction|UpdateSmogAppearance (Variables|SmogManagement|GetGoodSituationFog))
  (bind _asbp_push_button (Utilities|Casting|CastToBP_PushButton (Variables|/Script/Engine.ChildActorComponent|GetChildActor (Variables|Default|GetBP_LaunchGame))))
  (Variables|ObjectReference|SetLaunchGameButton%20Ref _asbp_push_button))

(fn ComputeAlpha
  (return (/ (Variables|Default|GetNumber%20of%20Succeeded%20machines) (Variables|Default|GetNumber%20of%20enables%20machines))))

(fn DefineReferences
  (bind _returnvalue (SaveGame|LoadGamefromSlot "CurrentGame"))
  (bind _asbp_save_territory_data (Utilities|Casting|CastToBP_SaveTerritoryData _returnvalue)
    (:then
      (Variables|Objectreference|SetPersistentGameDataRef _asbp_save_territory_data))
    (:CastFailed
      (Development|PrintString "Unable to retrieve game data of the save
It continues anyway without correct territory data" true true "(R=1.000000,G=0.293411,B=0.000000,A=1.000000)" 4.0 "territory data")))
  (bind _asmain_game_mode (Utilities|Casting|CastToMainGameMOde (Game|GetGameMode)))
  (Variables|ObjectReference|SetGame%20Mode%20Ref _asmain_game_mode)
  ;[0 0 0] Ref Climate Data Screen
  (bind _asw_bridge_scanner_status (Utilities|Casting|CastToW_Bridge_ScannerStatus (UserInterface|GetWidget (Variables|Default|GetScannerStatus))))
  (Variables|ObjectReference|SetBridge%20Scanner%20Status%20Ref _asw_bridge_scanner_status)
  ;[0 0 0] Ref Climate Data Screen
  (bind _asw_bridge_climate_data (Utilities|Casting|CastToW_Bridge_ClimateData (UserInterface|GetWidget (Variables|Default|GetClimateImpacts))))
  (Variables|ObjectReference|SetAs%20W%20Bridge%20Climate%20Data _asw_bridge_climate_data)
  ;[0 0 0] Ref Machine Reader Screen
  (bind _asw_bridge_machine_screen (Utilities|Casting|CastToW_Bridge_MachineScreen (UserInterface|GetWidget (Variables|Default|GetMachineScreen))))
  (Variables|ObjectReference|SetAs%20W%20Bridge%20Machine%20Screen _asw_bridge_machine_screen)
  ;[0 0 0] Ref Main Screen
  (bind _asw_bridge_main_screen (Utilities|Casting|CastToW_Bridge_MainScreen (UserInterface|GetWidget (Variables|Default|GetMainScreen))))
  (Variables|ObjectReference|SetMainScreen%20ref _asw_bridge_main_screen)
  ;[0 0 0] Agri widget
  (bind _asw_machine_status (Utilities|Casting|CastToW_MachineStatus (UserInterface|GetWidget (Variables|Default|GetAgriculture%20Machine%20Details))))
  (Variables|MachineStateWidgets|SetAgriMachineWidget%20ref _asw_machine_status)
  ;[0 0 0] Mobility
  (bind _asw_machine_status_2 (Utilities|Casting|CastToW_MachineStatus (UserInterface|GetWidget (Variables|Default|GetMobility%20Machine%20Details))))
  (Variables|MachineStateWidgets|SetMobilityMachineWidget%20ref _asw_machine_status_2)
  ;[0 0 0] Energy machine
  (bind _asw_machine_status_3 (Utilities|Casting|CastToW_MachineStatus (UserInterface|GetWidget (Variables|Default|GetEnergy%20Machine%20Details))))
  (Variables|MachineStateWidgets|SetEnergyMachineWidget%20ref _asw_machine_status_3)
  ;[0 0 0] Industry
  (bind _asw_machine_status_4 (Utilities|Casting|CastToW_MachineStatus (UserInterface|GetWidget (Variables|Default|GetIndustry%20Machine%20Details))))
  (Variables|MachineStateWidgets|SetIndustryMachineWidget%20%20ref _asw_machine_status_4)
  ;[0 0 0] Residential
  (bind _asw_machine_status_5 (Utilities|Casting|CastToW_MachineStatus (UserInterface|GetWidget (Variables|Default|GetResidential%20Machine%20Details))))
  (Variables|MachineStateWidgets|SetResidentialMachineWidget%20%20ref _asw_machine_status_5))

(fn UpdateMachineStatusWidget
  (params (Machine%20status%20widget%20 :type W%20Machine%20Status%20Object%20Reference) (Machine%20succeeded? :type Boolean) (Machine%20Name :type Text) (Pollutants :type S%20Territory%20Emissions%20Sector%20Specific%20Structure))
  (Default|SetMachineName Machine%20status%20widget%20 Machine%20Name)
  (if Machine%20succeeded?
    (Default|SetMachineMessage Machine%20status%20widget%20 true)
    (Default|SetMachineStatusLogotoValid Machine%20status%20widget%20))
  (Default|UpdatePollutantValues Machine%20status%20widget%20 Pollutants))